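; AI controller for the dog, running its behavior tree on the dog behavior blackboard.
; On BeginPlay it sets up the blackboard and starts the tree, then writes the IsOwnerClose key every Tick from a range-check function.
; That function currently always returns true; a player-to-pawn distance comparison sits unused beside it.
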(event EventBeginPlay
  (bind _blackboardcomponent (Class|AIController|UseBlackboard "/Game/AI/Krishna/DogAI/BB_DogBehavior.BB_DogBehavior"))
  (Variables|Default|SetBlackBoardComponent _blackboardcomponent)
  (AI|RunBehaviorTree "/Game/AI/Krishna/DogAI/BT_DogBehavior.BT_DogBehavior"))

(event EventTick
  (params (DeltaSeconds :type Float%20%28single-precision%29))
  (AI|Components|Blackboard|SetValueasBool (Variables|Default|GetBlackBoardComponent) (Variables|Default|GetIsOwnerClose) (CallFunction|IsOwnderinRange)))

(fn ConstructionScript)

(fn IsOwnderinRange
  (return true))