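; Wolf player character that moves relative to camera yaw and turns its head toward the control rotation, with multiplayer support.
; Forward input ignores backing up, and sideways input always blends in forward motion.
; The server stores control yaw in a manually replicated variable; every Tick eases the ABP_WolfTut head angle toward its offset from actor yaw, printing debug values.
; An unused base-aim-rotation alternative remains, and LookUp also drives yaw.
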(event EventTick
  (params (DeltaSeconds :type Float%20%28single-precision%29))
  (if (Ability|HasAuthority)
    (Variables|Default|SetReplicatedRotaion (.yaw (Pawn|GetControlRotation :!class /Script/Engine.Pawn)))
    (CallFunction|UpdateHeadRotation DeltaSeconds)
    (else
      (CallFunction|UpdateHeadRotation DeltaSeconds))))

(event Input|AxisEvents|InputAxisMoveForward
  (params (AxisValue :type Float%20%28single-precision%29))
  (Pawn|Input|AddMovementInput (Math|Vector|GetForwardVector (Math|Rotator|MakeRotator 0.0 0.0 (.yaw (Pawn|GetControlRotation :!class /Script/Engine.Pawn)))) (Math|Float|Clamp(Float) AxisValue) false))

(event Input|AxisEvents|InputAxisMoveRight
  (params (AxisValue :type Float%20%28single-precision%29))
  (Pawn|Input|AddMovementInput (Math|Vector|Normalize (+ (* (Math|Vector|GetRightVector (Math|Rotator|MakeRotator 0.0 0.0 (.yaw (Pawn|GetControlRotation :!class /Script/Engine.Pawn)))) AxisValue) (Math|Vector|GetForwardVector (Math|Rotator|MakeRotator 0.0 0.0 (.yaw (Pawn|GetControlRotation :!class /Script/Engine.Pawn)))))) (Math|Float|Absolute(Float) AxisValue) false))

(event Input|AxisEvents|InputAxisTurn
  (params (AxisValue :type Float%20%28single-precision%29))
  (Pawn|Input|AddControllerYawInput AxisValue))

(event Input|AxisEvents|InputAxisLookUp
  (params (AxisValue :type Float%20%28single-precision%29))
  (Pawn|Input|AddControllerYawInput AxisValue))

(fn ConstructionScript)

(fn UpdateHeadRotation
  (params (DeltaTIme :type Float%20%28double-precision%29))
  (bind _replicatedrotaion (Variables|Default|GetReplicatedRotaion))
  (bind _asabp_wolf_tut (Utilities|Casting|CastToABP_WolfTut (Components|SkeletalMesh|GetAnimInstance (Variables|Character|GetMesh))))
  (Variables|Default|SetAnimationRef _asabp_wolf_tut)
  ;[1 1 1] Manually replicarted control rotation
  (bind _output_get (Variables|/Game/TurningCircleVideo/ABP_WolfTut.ABP_WolfTut_C|SetHeadRotChar (Variables|Default|GetAnimationRef) (Math|Interpolation|FInterpTo (Variables|/Game/TurningCircleVideo/ABP_WolfTut.ABP_WolfTut_C|GetHeadRotChar (Variables|Default|GetAnimationRef)) (Math|Float|ClampAngle (- _replicatedrotaion (.yaw (Transformation|GetActorRotation))) -179.9 1.8e+02) DeltaTIme 3.0)))
  (Development|PrintString (Utilities|String|ToString(Float) _output_get) true true "(R=0.000000,G=0.660000,B=1.000000,A=1.000000)" DeltaTIme)
  (Development|PrintString (Utilities|String|ToString(Float) _replicatedrotaion) true true "(R=0.000000,G=0.660000,B=1.000000,A=1.000000)" DeltaTIme))

(fn BasetoControlRotation
  (params (YAWIn :type Float%20%28double-precision%29))
  (if (>= YAWIn 1.8e+02)
    (return (- YAWIn 3.6e+02))
    (else
      (return YAWIn))))